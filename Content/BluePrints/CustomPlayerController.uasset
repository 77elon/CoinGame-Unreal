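; Custom player controller that sets up the HUD and provides a save-and-quit key.
; On BeginPlay it adds the coin, level notice and notice widgets to the viewport, caches the NewGameInstance and creates a fresh MenuSaveGame object without loading existing data.
; Pressing Q copies coin, level and life values from the game instance into that object, saves it to a fixed slot, prints a confirmation and quits after a short delay.
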(event EventBeginPlay
  (Utilities|FlowControl|Sequence
    (:then_0
      (bind _returnvalue (UserInterface|CreateWidget "/Game/UI/Widget_Coin.Widget_Coin_C"))
      (UserInterface|Viewport|AddtoViewport _returnvalue 0))
    (:then_1
      (bind _asnew_game_instance (Utilities|Casting|CastToNewGameInstance (Game|GetGameInstance)))
      (Variables|Default|SetGameInstance _asnew_game_instance))
    (:then_2
      (bind _returnvalue_2 (SaveGame|CreateSaveGameObject "/Game/BluePrints/MenuSaveGame.MenuSaveGame_C"))
      (Variables|Default|SetMenuSaveGame _returnvalue_2))
    (:then_3
      (bind _returnvalue_3 (UserInterface|CreateWidget "/Game/UI/Level_Notice.Level_Notice_C"))
      (UserInterface|Viewport|AddtoViewport _returnvalue_3 2))
    (:then_4
      (bind _returnvalue_4 (UserInterface|CreateWidget "/Game/UI/Notice.Notice_C"))
      (UserInterface|Viewport|AddtoViewport _returnvalue_4 0))))

(event Input|KeyboardEvents|Q
  (params (Key :type Key%20Structure :default "None"))
  (bind _menusavegame (Variables|Default|GetMenuSaveGame))
  (bind _gameinstance (Variables|Default|GetGameInstance))
  (:Pressed
    (Variables|/Game/BluePrints/MenuSaveGame.MenuSaveGame_C|SetCoinStorData _menusavegame (Variables|/Game/BluePrints/NewGameInstance.NewGameInstance_C|GetCoinStor _gameinstance))
    (Variables|/Game/BluePrints/MenuSaveGame.MenuSaveGame_C|SetLevelStorData _menusavegame (Variables|/Game/BluePrints/NewGameInstance.NewGameInstance_C|GetLevelStor _gameinstance))
    (Variables|/Game/BluePrints/MenuSaveGame.MenuSaveGame_C|SetLifeStorData _menusavegame (Variables|/Game/BluePrints/NewGameInstance.NewGameInstance_C|GetLifeStor _gameinstance))
    (SaveGame|SaveGametoSlot _menusavegame "A")
    (Development|PrintString "Game Saved!!")
    (Utilities|FlowControl|Delay 0.25)
    (Game|QuitGame 0 "Quit" false)))

(fn ConstructionScript)