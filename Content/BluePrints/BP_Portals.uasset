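; BP_Portals is a level exit portal that sends the player on to the next level once the current one is cleared.
; On BeginPlay it records its CurrentLevel in the NewGameInstance's LevelStor.
; When a ThirdPersonCharacter overlaps its sphere, it checks LevelClear on the game state.
; If set, it slows global time, waits briefly and opens NextLevel by name.
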(event OnComponentBeginOverlap(Sphere)
  (params (OverlappedComponent :type Primitive%20Component%20Object%20Reference) (OtherActor :type Actor%20Object%20Reference) (OtherComp :type Primitive%20Component%20Object%20Reference) (OtherBodyIndex :type Integer) (bFromSweep :type Boolean) (SweepResult :type Hit%20Result%20Structure%20%28by%20ref%29))
  (Utilities|Casting|CastToThirdPersonCharacter OtherActor)
  (bind _asnew_game_state_base (Utilities|Casting|CastToNewGameStateBase (Game|GetGameState)))
  (if (Variables|/Game/BluePrints/NewGameStateBase.NewGameStateBase_C|GetLevelClear _asnew_game_state_base)
    (Utilities|Time|SetGlobalTimeDilation 0.5)
    (Utilities|FlowControl|Delay 0.5)
    (Game|OpenLevel(byName) (Variables|Default|GetNextLevel))))

(event EventBeginPlay
  (bind _asnew_game_instance (Utilities|Casting|CastToNewGameInstance (Game|GetGameInstance)))
  (Variables|/Game/BluePrints/NewGameInstance.NewGameInstance_C|SetLevelStor _asnew_game_instance (Variables|Default|GetCurrent_Level)))

(fn ConstructionScript)