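; BP_Pickup is a coin pickup that the player collects by walking into its sphere.
; BeginPlay caches references to the NewGameStateBase game state and the NewGameInstance game instance.
; On overlap with a ThirdPersonCharacter, it adds CoinValue to both the character's Coins and the game instance's CoinStor.
; It then calls CoinTest on the game state and destroys itself.
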(event OnComponentBeginOverlap(Sphere)
  (params (OverlappedComponent :type Primitive%20Component%20Object%20Reference) (OtherActor :type Actor%20Object%20Reference) (OtherComp :type Primitive%20Component%20Object%20Reference) (OtherBodyIndex :type Integer) (bFromSweep :type Boolean) (SweepResult :type Hit%20Result%20Structure%20%28by%20ref%29))
  (bind _gameinstance (Variables|Default|GetGameInstance))
  (bind _asthird_person_character (Utilities|Casting|CastToThirdPersonCharacter OtherActor))
  (Variables|/Game/ThirdPersonBP/Blueprints/ThirdPersonCharacter.ThirdPersonCharacter_C|SetCoins _asthird_person_character (+ (Variables|/Game/ThirdPersonBP/Blueprints/ThirdPersonCharacter.ThirdPersonCharacter_C|GetCoins _asthird_person_character) (Variables|Default|GetCoinValue)))
  (Variables|/Game/BluePrints/NewGameInstance.NewGameInstance_C|SetCoinStor _gameinstance (+ (Variables|/Game/BluePrints/NewGameInstance.NewGameInstance_C|GetCoinStor _gameinstance) (Variables|Default|GetCoinValue)))
  (Default|CoinTest (Variables|Default|GetGameState))
  (Actor|DestroyActor))

(event EventBeginPlay
  (Utilities|FlowControl|Sequence
    (:then_0
      (bind _asnew_game_state_base (Utilities|Casting|CastToNewGameStateBase (Game|GetGameState)))
      (Variables|Default|SetGameState _asnew_game_state_base))
    (:then_1
      (bind _asnew_game_instance (Utilities|Casting|CastToNewGameInstance (Game|GetGameInstance)))
      (Variables|Default|SetGameInstance _asnew_game_instance))))

(fn ConstructionScript)