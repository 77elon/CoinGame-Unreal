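; Char1 is an armed character that fires hitscan shots at the player through its AutoFire event.
; A Camera-channel line trace runs from its arrow component toward the player, playing a small explosion effect and sound on any blocking hit.
; Hits on the player spawn sparks and decrement life stored in the GameInstance.
; At zero life it shows a Notice widget, then resets life and coins and opens a level.
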(event Custom|AutoFire
  (bind _arrow1 (Variables|Default|GetArrow1))
  (bind _returnvalue (Transformation|GetWorldLocation _arrow1))
  (bind _asthird_person_character (Utilities|Casting|CastToThirdPersonCharacter (Game|Player|GetPlayerPawn 0)))
  (Variables|Default|SetPawn _asthird_person_character)
  (bind (_outhit _returnvalue_2) (Collision|LineTraceByChannel _returnvalue (+ (Transformation|GetWorldLocation (Variables|/Script/Engine.Actor|GetRootComponent (Variables|Default|GetPawn))) "0,0.000000,50.000000") "TraceTypeQuery2" false 0 "None"))
  (if _returnvalue_2
    (Effects|SpawnEmitteratLocation "/Game/StarterContent/Particles/P_Explosion.P_Explosion" _returnvalue "0, 0, 0" "0.100000,0.100000,0.100000" true "AutoRelease")
    (Audio|PlaySoundatLocation "/Game/StarterContent/Audio/Explosion01.Explosion01" _returnvalue "0, 0, 0" 0.2 0.5 0.0 0 0 0)
    (if (== (.HitActor (Collision|BreakHitResult _outhit)) (Variables|Default|GetPawn))
      (Effects|SpawnEmitterAttached "/Game/StarterContent/Particles/P_Sparks.P_Sparks" (Variables|/Script/Engine.Character|GetMesh (Variables|Default|GetPawn)) "None" (.Location (Collision|BreakHitResult _outhit)) "0, 0, 0" "0.100000,0.100000,0.100000" "KeepWorldPosition" true "AutoRelease")
      (bind _asnew_game_instance (Utilities|Casting|CastToNewGameInstance (Game|GetGameInstance)))
      (bind _output_get (Variables|/Game/BluePrints/NewGameInstance.NewGameInstance_C|SetLifeStor _asnew_game_instance (- (Variables|/Game/BluePrints/NewGameInstance.NewGameInstance_C|GetLifeStor _asnew_game_instance) 1)))
      (if (< _output_get 1)
        (bind _returnvalue_3 (UserInterface|CreateWidget "/Game/UI/Notice.Notice_C"))
        (Variables|/Game/UI/Notice.Notice_C|SetCheckPoint _returnvalue_3 true)
        (UserInterface|Viewport|AddtoViewport _returnvalue_3 0)
        (Utilities|FlowControl|Delay 2.0)
        (bind _asnew_game_instance_2 (Utilities|Casting|CastToNewGameInstance (Game|GetGameInstance)))
        (Variables|/Game/ThirdPersonBP/Blueprints/ThirdPersonCharacter.ThirdPersonCharacter_C|SetCoins (Variables|Default|GetPawn) 0)
        (Variables|/Game/BluePrints/NewGameInstance.NewGameInstance_C|SetLifeStor _asnew_game_instance_2 10)
        (Variables|/Game/BluePrints/NewGameInstance.NewGameInstance_C|SetCoinStor _asnew_game_instance_2 0)
        (Game|OpenLevel(byName) (Variables|Default|GetLevel))))))

(fn ConstructionScript)